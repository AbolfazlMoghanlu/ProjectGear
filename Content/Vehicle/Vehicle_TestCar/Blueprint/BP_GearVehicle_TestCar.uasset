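; BP_GearVehicle_TestCar is a test car vehicle Blueprint that keeps its wheel meshes in step with the inherited wheel data.
; After the parent Tick, it loops over Wheels and finds each static mesh component by a tag matching the wheel's name.
; It moves that mesh to the wheel's world transform, composed with a world-Z offset from rest length, suspension offset and wheel radius.
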(event EventBeginPlay
  (|CallParentFunction) ; This node is disabled and will not be called.\nDrag off pins to build functionality.
)

(event Collision|EventActorBeginOverlap
  (params (OtherActor :type Actor%20Object%20Reference))
  (|CallParentFunction OtherActor) ; This node is disabled and will not be called.\nDrag off pins to build functionality.
)

(event EventTick
  (params (DeltaSeconds :type Float%20%28single-precision%29))
  (|CallParentFunction DeltaSeconds)
  (for _array_element (Variables|Default|GetWheels)
    (if (Utilities|Array|IsValidIndex (Actor|GetComponentsbyTag "/Script/Engine.StaticMeshComponent" (.WheelName (Utilities|Struct|BreakGearWheel _array_element))))
      (Transformation|SetWorldTransform (Utilities|Array|Get(acopy) (Actor|GetComponentsbyTag "/Script/Engine.StaticMeshComponent" (.WheelName (Utilities|Struct|BreakGearWheel _array_element)))) (Math|Transform|ComposeTransforms (.WorldTransform (Utilities|Struct|BreakGearWheel _array_element)) (Math|Transform|MakeTransform (Math|Vector|MakeVector 0.0 0.0 (+ (* (.RestLength (Utilities|Struct|BreakGearWheel _array_element)) -1.0) (.SuspentionOffset (Utilities|Struct|BreakGearWheel _array_element)) (.WheelRadius (Utilities|Struct|BreakGearWheelData (.WheelData (Utilities|Struct|BreakGearWheel _array_element)))))))) false false))))

(fn ConstructionScript
  (|CallParentFunction))